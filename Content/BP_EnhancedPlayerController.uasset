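; Player controller that creates the HUD and handles button and key input for a game-state counter and bomb spawning.
; On BeginPlay it adds BPW_HUD to the viewport, and OnButtonClicked calls IncreaseVariable on BP_EnhancedGameState.
; The 1 key calls SpawnBomb, which spawns a Bomb at a stored transform only with authority.
; SetBPDoor stores a Door reference that is not otherwise used here.
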(event `self.ReceiveBeginPlay`
  ;[1 1 1] Comment
  (bind _returnvalue (`|CreateWidget` "/Game/BPW_HUD.BPW_HUD_C"))
  (`UserWidget.AddToViewport` _returnvalue 0))

(event `OnButtonClicked`
  ;[1 1 1] Comment
  (bind _asbp_enhanced_game_state (cast `/Game/BP_EnhancedGameState` (`GameplayStatics.GetGameState`)))
  (`/Game/BP_EnhancedGameState.IncreaseVariable` _asbp_enhanced_game_state))

(event `Key|One`
  (params (Key :type "Key Structure"))
  (:`Pressed`
    (`self.SpawnBomb`)))

(event `SpawnBomb`
  (`/Engine/EditorBlueprintResources/ActorMacros.Switch Has Authority`
    (:`Authority`
      (`|SpawnActorFromClass` (`self.Bomb`) (`self.NewVar_3`) "Undefined" "OverrideRootScale" null null))))

(fn `SetBPDoor`
  (params (NewParam :type "/Game/BP_Door Object Reference"))
  (set `self.Door` NewParam))

(fn `UserConstructionScript`)