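; BP_EnhancedGameMode is a multiplayer game mode that tracks joining players and reads a player limit.
; PostLogin appends each new controller to PlayerControllerList, and BeginPlay parses MaxNumPlayers from the options string, though nothing here uses it.
; ReadyToStartMatch and OnStartMatch are empty.
; A two-player readiness check, StartMatch call and level-open call are left disconnected.
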(event `self.K2_PostLogin`
  (params (NewPlayer :type "PlayerController Object Reference"))
  ;[1 1 1] Fired After player controller is connected
  (`KismetArrayLibrary.Array_Add` (`self.PlayerControllerList`) NewPlayer))

(event `OnStartMatch`)

(event `self.ReceiveBeginPlay`
  (set `self.MaxNumPlayers` (`KismetStringLibrary.Conv_StringToInt` (`GameplayStatics.ParseOption` (`self.OptionsString`) "MaxNumPlayers"))))

(fn `ReadyToStartMatch`
  (returns (ReturnValue :type Boolean)))

(fn `UserConstructionScript`)