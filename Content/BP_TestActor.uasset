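; BP_TestActor is a network test actor that exercises authority checks and RPC-style events through a text render display.
; A looping authority-side timer drains Health, and Tick shows the value until StopTick is set.
; Box begin overlap sets StopTick on authority and fires a multicast text change.
; End overlap sets StopTick without an authority check and calls the client event to change the text, while the server event is an empty, uncalled stub.
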(event `self.Box.OnComponentEndOverlap`
  (params (OverlappedComponent :type "PrimitiveComponent Object Reference") (OtherActor :type "Actor Object Reference") (OtherComp :type "PrimitiveComponent Object Reference") (OtherBodyIndex :type Integer))
  ;[0.2994 0.4422 1] Run On Server - called by client and runs only on server
  (set `self.StopTick` true)
  (`self.RunOnClientEvent`))

(event `RunOnServerEvent`
  ;[0.2994 0.4422 1] Run On Server - called by client and runs only on server
)

(event `RunOnClientEvent`
  ;[0.2994 0.4422 1] Run On Server - called by client and runs only on server
  (`TextRenderComponent.K2_SetText` (`self.TextRender`) (`self.NewVar_1`)))

(event `self.Box.OnComponentBeginOverlap`
  (params (OverlappedComponent :type "PrimitiveComponent Object Reference") (OtherActor :type "Actor Object Reference") (OtherComp :type "PrimitiveComponent Object Reference") (OtherBodyIndex :type Integer) (bFromSweep :type Boolean) (SweepResult :type "HitResult Structure (by ref)"))
  ;[0.6477 1 0.431] Multicast - runs on the server and then forwarded automatically to clients
  (`/Engine/EditorBlueprintResources/ActorMacros.Switch Has Authority`
    (:`Authority`
      (set `self.StopTick` true)
      (`self.TriggerFireMulticast`))))

(event `TriggerFireMulticast`
  ;[0.6477 1 0.431] Multicast - runs on the server and then forwarded automatically to clients
  (`TextRenderComponent.K2_SetText` (`self.TextRender`) (`self.NewVar_0`)))

(event `self.ReceiveBeginPlay`
  ;[1 1 1] Comment
  (`/Engine/EditorBlueprintResources/ActorMacros.Switch Has Authority`
    (:`Authority`
      (`KismetSystemLibrary.K2_SetTimerDelegate` (delegate `CustomEvent_0`) 1.0 true))))

(event `CustomEvent_0`
  ;[1 1 1] Comment
  (set `self.Health` (- (`self.Health`) 10)))

(event `self.ReceiveTick`
  (params (DeltaSeconds :type "Float (single-precision)"))
  ;[1 1 1] Tick
  (if (not (`self.StopTick`))
    (`TextRenderComponent.K2_SetText` (`self.TextRender`) (`KismetTextLibrary.Conv_StringToText` (`KismetStringLibrary.BuildString_Int` "" "Health : " (`self.Health`))))))

(fn `UserConstructionScript`)