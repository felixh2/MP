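; BP_Enemy is an enemy Blueprint that watches its HP value for changes and raises a change notification.
; On BeginPlay it caches HP and starts a looping timer that polls several times a second.
; When the value differs from the cached one, it calls the OnHPChanged dispatcher and updates the cache, so detection is polled instead of fired where HP is set.
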(event `self.ReceiveBeginPlay`
  (set `self.PrevHP` (`self.HP`))
  (`KismetSystemLibrary.K2_SetTimerDelegate` (delegate `CustomEvent_0`) 0.2 true))

(event `CustomEvent_0`
  (if (!= (`self.HP`) (`self.PrevHP`))
    (`self.OnHPChanged`)
    (set `self.PrevHP` (`self.HP`))))

(fn `UserConstructionScript`)