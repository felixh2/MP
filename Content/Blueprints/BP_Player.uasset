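; Player Blueprint that watches its Insanity value and broadcasts when it changes.
; BeginPlay caches the starting value and starts a looping timer that polls five times a second.
; Each tick of the timer compares Insanity to the cached value, calls OnInsanityChange on any difference, then updates the cache.
; Nothing in this graph modifies Insanity itself.
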(event `self.ReceiveBeginPlay`
  (set `self.PrevInsanity` (`self.Insanity`))
  (`KismetSystemLibrary.K2_SetTimerDelegate` (delegate `CustomEvent_0`) 0.2 true))

(event `CustomEvent_0`
  (if (!= (`self.Insanity`) (`self.PrevInsanity`))
    (`self.OnInsanityChange`)
    (set `self.PrevInsanity` (`self.Insanity`))))

(fn `UserConstructionScript`)